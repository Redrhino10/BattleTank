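; Tank Blueprint that handles camera orbit input for aiming.
; The AimBarrelX axis yaws the Gimbal and AimBarrelY pitches the SpringArm, splitting the two rotations across separate components.
; Both apply local rotation scaled by world delta seconds and RotationVariable for frame-rate-independent speed.
; The BeginPlay, overlap and Tick events are disabled stubs, and the construction script is empty.
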(event `InputAxis|AimBarrelX`
  (params (AxisValue :type "Float (single-precision)"))
  ;[1 1 1] Camera Input Binding
  (`SceneComponent.K2_AddLocalRotation` (`self.Gimbal`) (`KismetMathLibrary.MakeRotator` 0.0 0.0 (* AxisValue (`GameplayStatics.GetWorldDeltaSeconds`) (`self.RotationVariable`))) false false))

(event `InputAxis|AimBarrelY`
  (params (AxisValue :type "Float (single-precision)"))
  ;[1 1 1] Camera Input Binding
  (`SceneComponent.K2_AddLocalRotation` (`self.SpringArm`) (`KismetMathLibrary.MakeRotator` 0.0 (* AxisValue (`GameplayStatics.GetWorldDeltaSeconds`) (`self.RotationVariable`))) false false))

(fn `UserConstructionScript`)